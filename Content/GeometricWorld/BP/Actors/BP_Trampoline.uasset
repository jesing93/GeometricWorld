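; Trampoline actor that bounces the player character and BP_Block actors along its mesh's up vector at LaunchStrength.
; On overlap, the character is launched with its Z velocity overridden, with a jump sound if it was falling, while blocks get their physics linear velocity replaced.
; The construction script sets a cylinder or cube mesh from the Form setting.
; An impulse path for StaticMeshActors is present but never runs.
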(event OnComponentBeginOverlap(StaticMesh)
  (params (OverlappedComponent :type Primitive%20Component%20Object%20Reference) (OtherActor :type Actor%20Object%20Reference) (OtherComp :type Primitive%20Component%20Object%20Reference) (OtherBodyIndex :type Integer) (bFromSweep :type Boolean) (SweepResult :type Hit%20Result%20Structure%20%28by%20ref%29))
  (bind _returnvalue (Utilities|GetClass OtherActor))
  (bind _asbp_geometric_world_character (Utilities|Casting|CastToBP_GeometricWorldCharacter OtherActor))
  (if (== _returnvalue "/Game/GeometricWorld/BP/Character/BP_GeometricWorldCharacter.BP_GeometricWorldCharacter_C")
    (if (AI|Components|NavMovement|IsFalling (Variables|/Script/Engine.Character|GetCharacterMovement _asbp_geometric_world_character))
      (Audio|PlaySoundatLocation "/Game/GeometricWorld/SFX/Jump.Jump" (Transformation|GetActorLocation _asbp_geometric_world_character) "0, 0, 0" 1.0 1.0 0.0 0 0 0 0))
    (Character|LaunchCharacter _asbp_geometric_world_character (* (Math|Vector|GetUpVector (Variables|Default|GetStaticMesh)) (Variables|Default|GetLaunchStrength)) false true)
    (elif (== _returnvalue "/Game/GeometricWorld/BP/Actors/BP_Block.BP_Block_C")
      (Physics|SetPhysicsLinearVelocity (Variables|/Game/GeometricWorld/BP/Actors/BP_Block.BP_Block_C|GetStaticMesh (.AsBP%20Block (Utilities|Casting|CastToBP_Block OtherActor))) (* (Math|Vector|GetUpVector (Variables|Default|GetStaticMesh)) (Variables|Default|GetLaunchStrength)) false "None"))))

(event EventBeginPlay)

(event EventTick
  (params (DeltaSeconds :type Float%20%28single-precision%29)))

(fn ConstructionScript
  (bind _staticmesh (Variables|Default|GetStaticMesh))
  (switch Utilities|FlowControl|Switch|SwitchonPlainForms (Variables|Default|GetForm)
    (:NewEnumerator1
      (Components|StaticMesh|SetStaticMesh _staticmesh "/Game/GeometricWorld/StaticMeshes/BasicCylinder.BasicCylinder"))
    (:NewEnumerator0
      (Components|StaticMesh|SetStaticMesh _staticmesh "/Game/GeometricWorld/StaticMeshes/BasicCube.BasicCube"))))