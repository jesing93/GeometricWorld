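; BP_Puzzle is a button-combination puzzle actor that switches a Target on or off.
; Activate and Deactivate both run the same check: every button in CorrectButtons must be pressed and none in WrongButtons, with each loop breaking at the first failure.
; The result calls Activate on the Target when the combination is correct and Deactivate otherwise.
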(event EventActivate
  (bind _target (Variables|Default|GetTarget))
  (Variables|Default|SetCorrect? true)
  (bind _array_element (Utilities|Array|ForEachLoopwithBreak (Variables|Default|GetCorrectButtons) :!label _label)
    (:LoopBody
      (if (not (Variables|/Game/GeometricWorld/BP/Actors/BP_Button.BP_Button_C|GetPressed _array_element))
        (Variables|Default|SetCorrect? false)
        (goto _label Break)))
    (:Completed
      (bind _array_element_2 (Utilities|Array|ForEachLoopwithBreak (Variables|Default|GetWrongButtons) :!label _label_2)
        (:LoopBody
          (if (Variables|/Game/GeometricWorld/BP/Actors/BP_Button.BP_Button_C|GetPressed _array_element_2)
            (Variables|Default|SetCorrect? false)
            (goto _label_2 Break)))
        (:Completed
          (if (Variables|Default|GetCorrect?)
            (Default|Activate _target)
            (else
              (Default|Deactivate _target))))))))

(event EventDeactivate
  (bind _target (Variables|Default|GetTarget))
  (Variables|Default|SetCorrect? true)
  (bind _array_element (Utilities|Array|ForEachLoopwithBreak (Variables|Default|GetCorrectButtons) :!label _label)
    (:LoopBody
      (if (not (Variables|/Game/GeometricWorld/BP/Actors/BP_Button.BP_Button_C|GetPressed _array_element))
        (Variables|Default|SetCorrect? false)
        (goto _label Break)))
    (:Completed
      (bind _array_element_2 (Utilities|Array|ForEachLoopwithBreak (Variables|Default|GetWrongButtons) :!label _label_2)
        (:LoopBody
          (if (Variables|/Game/GeometricWorld/BP/Actors/BP_Button.BP_Button_C|GetPressed _array_element_2)
            (Variables|Default|SetCorrect? false)
            (goto _label_2 Break)))
        (:Completed
          (if (Variables|Default|GetCorrect?)
            (Default|Activate _target)
            (else
              (Default|Deactivate _target))))))))

(fn ConstructionScript
  (|CallParentFunction))