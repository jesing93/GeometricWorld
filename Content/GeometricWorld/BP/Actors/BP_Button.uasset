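; BP_Button is a pressure button that switches other actors when something overlaps its box.
; A press recolors and sinks the button, plays a sound, activates Target actors and deactivates ReverseTarget actors.
; With Hold set, emptying the box releases it, but only TriggerOnDeactivate inverts those calls and raises the button.
; Its own Activate and Deactivate events change state, material and position without propagating to targets.
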(event OnComponentBeginOverlap(Box)
  (params (OverlappedComponent :type Primitive%20Component%20Object%20Reference) (OtherActor :type Actor%20Object%20Reference) (OtherComp :type Primitive%20Component%20Object%20Reference) (OtherBodyIndex :type Integer) (bFromSweep :type Boolean) (SweepResult :type Hit%20Result%20Structure%20%28by%20ref%29))
  (if (not (Variables|Default|GetPressed))
    (Variables|Default|SetPressed true)
    (Rendering|Material|SetMaterial (Variables|Default|GetButton) 0 "/Game/GeometricWorld/Materials/MI_BasicMaterialEmmisivePurple.MI_BasicMaterialEmmisivePurple")
    (Audio|PlaySoundatLocation "/Game/GeometricWorld/SFX/Button.Button" (Transformation|GetActorLocation) "0, 0, 0" 1.0 1.0 0.0 "/Game/GeometricWorld/SFX/SA_Standard.SA_Standard" 0 0 0)
    (for _array_element (Variables|Default|GetTarget)
      (Default|Activate _array_element))
    (for _array_element_2 (Variables|Default|GetReverseTarget)
      (Default|Deactivate _array_element_2))
    (Components|MoveComponentTo (Variables|Default|GetButton) (- (Variables|Default|GetStartingLocation) "0.000000,0.000000,4.000000") "0, 0, 0" true false 0.2 false)))

(event OnComponentEndOverlap(Box)
  (params (OverlappedComponent :type Primitive%20Component%20Object%20Reference) (OtherActor :type Actor%20Object%20Reference) (OtherComp :type Primitive%20Component%20Object%20Reference) (OtherBodyIndex :type Integer))
  (if (Math|Boolean|ANDBoolean (Variables|Default|GetPressed) (Variables|Default|GetHold) (== (Utilities|Array|Length (Collision|GetOverlappingActors (Variables|Default|GetBox) 0 :!class /Script/Engine.PrimitiveComponent)) 0))
    (Variables|Default|SetPressed false)
    (Rendering|Material|SetMaterial (Variables|Default|GetButton) 0 "/Game/GeometricWorld/Materials/MI_BasicMaterialEmmisiveOrange.MI_BasicMaterialEmmisiveOrange")
    (Audio|PlaySoundatLocation "/Game/GeometricWorld/SFX/Button.Button" (Transformation|GetActorLocation) "0, 0, 0" 1.0 0.75 0.0 "/Game/GeometricWorld/SFX/SA_Standard.SA_Standard" 0 0 0)
    (if (Variables|Default|GetTriggerOnDeactivate?)
      (for _array_element (Variables|Default|GetTarget)
        (Default|Deactivate _array_element))
      (for _array_element_2 (Variables|Default|GetReverseTarget)
        (Default|Activate _array_element_2))
      (Components|MoveComponentTo (Variables|Default|GetButton) (Variables|Default|GetStartingLocation) "0, 0, 0" true true 0.2 false))))

(event EventBeginPlay
  (Variables|Default|SetStartingLocation (Variables|/Script/Engine.SceneComponent|GetRelativeLocation (Variables|Default|GetButton)))
  (if (Variables|Default|GetPressed)
    (Rendering|Material|SetMaterial (Variables|Default|GetButton) 0 "/Game/GeometricWorld/Materials/MI_BasicMaterialEmmisivePurple.MI_BasicMaterialEmmisivePurple")
    (Components|MoveComponentTo (Variables|Default|GetButton) (- (Variables|Default|GetStartingLocation) "0.000000,0.000000,4.000000") "0, 0, 0" true false 0.2 false)))

(event EventActivate
  (Variables|Default|SetPressed true)
  (Rendering|Material|SetMaterial (Variables|Default|GetButton) 0 "/Game/GeometricWorld/Materials/MI_BasicMaterialEmmisivePurple.MI_BasicMaterialEmmisivePurple")
  (Components|MoveComponentTo (Variables|Default|GetButton) (- (Variables|Default|GetStartingLocation) "0.000000,0.000000,4.000000") "0, 0, 0" true false 0.2 false))

(event EventDeactivate
  (Variables|Default|SetPressed false)
  (Rendering|Material|SetMaterial (Variables|Default|GetButton) 0 "/Game/GeometricWorld/Materials/MI_BasicMaterialEmmisiveOrange.MI_BasicMaterialEmmisiveOrange")
  (Components|MoveComponentTo (Variables|Default|GetButton) (Variables|Default|GetStartingLocation) "0, 0, 0" true true 0.2 false))

(fn ConstructionScript)