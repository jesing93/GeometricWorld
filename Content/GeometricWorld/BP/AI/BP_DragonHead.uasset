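; BP_DragonHead is an enemy AI pawn that patrols the map, chases the player once detected, and kills them on overlap.
; Patrol walks to random reachable points, while Detect switches to AIMoveTo pursuit, alerting the player character and tilting the eyebrows.
; Tick resumes patrol when detection goes stale, with difficulty setting chase speed and follow time.
; A looping timer oscillates the jaws alongside an attached proximity sound.
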(event OnComponentBeginOverlap(Overlap)
  (params (OverlappedComponent :type Primitive%20Component%20Object%20Reference) (OtherActor :type Actor%20Object%20Reference) (OtherComp :type Primitive%20Component%20Object%20Reference) (OtherBodyIndex :type Integer) (bFromSweep :type Boolean) (SweepResult :type Hit%20Result%20Structure%20%28by%20ref%29))
  (bind _returnvalue (Game|GetPlayerCharacter 0))
  ;[1 1 1] Overlap player
  (if (== OtherActor _returnvalue)
    (Default|Death (.AsBP%20Geometric%20World%20Character (Utilities|Casting|CastToBP_GeometricWorldCharacter _returnvalue)))))

(event Custom|Patrol
  ;[1 1 1] Patrol map
  (if (not (Variables|Default|GetFollowing))
    (AI|AIMoveTo self (.RandomLocation (AI|Navigation|GetRandomReachablePointinRadius (Transformation|GetActorLocation) 2e+03 0 0)) 0 1e+01 true
      (:OnSuccess
        _)
      (:OnFail
        _))
    (Utilities|FlowControl|RetriggerableDelay 0.2)
    (CallFunction|Patrol)))

(event Custom|Follow
  ;[1 1 1] Follow player
  (if (Variables|Default|GetFollowing)
    (AI|AIMoveTo self "0, 0, 0" (Game|GetPlayerCharacter 0) 0.0 true
      (:OnFail
        (CallFunction|Follow)))))

(event Custom|Detect
  (params (Goal :type Actor%20Object%20Reference))
  ;[1 1 1] Detection event
  (Variables|Default|SetLastDetect (Utilities|Time|GetGameTimeinSeconds))
  (if (not (Variables|Default|GetFollowing))
    (Audio|PlaySound2D "/Game/GeometricWorld/SFX/Detected.Detected" 1.0 1.0 0.0 0 0)
    (Variables|Default|SetFollowing true)
    (Variables|/Script/Engine.CharacterMovementComponent|SetMaxWalkSpeed (Variables|Character|GetCharacterMovement) (CallFunction|FollowSpeed))
    (CallFunction|Follow)
    (Default|StartChase (.AsBP%20Geometric%20World%20Character (Utilities|Casting|CastToBP_GeometricWorldCharacter (Game|GetPlayerCharacter 0))))
    (Transformation|AddRelativeRotation (Variables|Default|GetLeftEyebrow) "40.000000,0.000000,0.000000" false false)))

(event Custom|MoveMouth
  (bind _loweryaw (Variables|Default|GetLowerYaw))
  (bind _relativelocation (Variables|/Script/Engine.SceneComponent|GetRelativeLocation _loweryaw))
  (bind _z (Math|Vector|BreakVector _relativelocation))
  ;[1 1 1] Mouth animation
  (if (Variables|Default|GetClosing?)
    (if (>= _z (+ (Variables|Default|GetLJawLocation) (Variables|Default|GetMouthMax)))
      (Variables|Default|SetClosing? false)
      (else
        (Transformation|AddRelativeLocation (Variables|Default|GetUpperYaw) "0.000000,0.000000,-0.500000" false false)
        (Transformation|AddRelativeLocation (Variables|Default|GetLowerYaw) "0.000000,0.000000,1.000000" false false)))
    (elif (<= _z (Variables|Default|GetLJawLocation))
      (Variables|Default|SetClosing? true)
      (else
        (Transformation|AddRelativeLocation (Variables|Default|GetUpperYaw) "0.000000,0.000000,0.500000" false false)
        (Transformation|AddRelativeLocation (Variables|Default|GetLowerYaw) "0.000000,0.000000,-1.000000" false false)))))

(event EventBeginPlay
  ;[1 1 1] Close sound
  (switch int 0
    (:Default
      _)
    (:0
      (Variables|Default|SetAttenuation "/Game/GeometricWorld/SFX/SA_CloseLong.SA_CloseLong"))
    (:1
      (Variables|Default|SetAttenuation "/Game/GeometricWorld/SFX/SA_CloseMedium.SA_CloseMedium"))
    (:2
      (Variables|Default|SetAttenuation "/Game/GeometricWorld/SFX/SA_Close.SA_Close")))
  (bind _returnvalue (Audio|SpawnSoundAttached "/Game/GeometricWorld/SFX/EnemySound.EnemySound" (Variables|Default|GetUpperYaw) "None" "0, 0, 0" "0, 0, 0" "KeepRelativeOffset" true 1.0 1.0 0.0 "/Game/GeometricWorld/SFX/SA_Close.SA_Close" 0 false))
  (bind _output_get (Variables|Default|SetCloseSound _returnvalue))
  (Audio|Components|Audio|Play _output_get 0.0)
  ;[1 1 1] Mouth animation start
  (Variables|Default|SetLJawLocation (.Z (Math|Vector|BreakVector (Variables|/Script/Engine.SceneComponent|GetRelativeLocation (Variables|Default|GetLowerYaw)))))
  (Utilities|Time|SetTimerbyEvent (delegate Custom|MoveMouth) 0.05 true)
  ;[1 1 1] Delay before start patrolling
  (if (Variables|Default|GetPatrolFromStart?)
    (Utilities|FlowControl|Delay (Variables|Default|GetStartPatrolDelay))
    (CallFunction|Patrol)))

(event EventTick
  (params (DeltaSeconds :type Float%20%28single-precision%29))
  ;[1 1 1] Stop following
  (if (and (Variables|Default|GetFollowing) (> (Utilities|Time|GetGameTimeinSeconds) (+ (Variables|Default|GetLastDetect) (Variables|Default|GetFollowTime))))
    (Variables|Default|SetFollowing false)
    (Variables|/Script/Engine.CharacterMovementComponent|SetMaxWalkSpeed (Variables|Character|GetCharacterMovement) 3e+02)
    (CallFunction|Patrol)
    (Default|StopChase (.AsBP%20Geometric%20World%20Character (Utilities|Casting|CastToBP_GeometricWorldCharacter (Game|GetPlayerCharacter 0))))
    (Transformation|AddRelativeRotation (Variables|Default|GetLeftEyebrow) "-40.000000,0.000000,0.000000" false false)))

(fn ConstructionScript
  (switch int (Variables|/Game/GeometricWorld/BP/GI_GeometricWorld.GI_GeometricWorld_C|GetDifficulty (.AsGI%20Geometric%20World (Utilities|Casting|CastToGI_GeometricWorld (Game|GetGameInstance))))
    (:0
      (Variables|Default|SetFollowTime 3.0))
    (:1
      (Variables|Default|SetFollowTime 3.5))
    (:2
      (Variables|Default|SetFollowTime 4.0))))

(fn FollowSpeed
  (return (+ 5e+02 (* 75 (Variables|/Game/GeometricWorld/BP/GI_GeometricWorld.GI_GeometricWorld_C|GetDifficulty (.AsGI%20Geometric%20World (Utilities|Casting|CastToGI_GeometricWorld (Game|GetGameInstance))))))))