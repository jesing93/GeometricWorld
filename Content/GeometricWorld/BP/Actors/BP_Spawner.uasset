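; Spawner actor that creates a destructible block, block or dragon head at its own transform, on BeginPlay or whenever Activate is called.
; With ControlSpawned, Activate replaces the tracked actor; otherwise it spawns another and tracks only the latest.
; Deactivate destroys the tracked actor with a hit sound at its mesh.
; SpawnedActorDestroy respawns when ControlSpawned and AutoRespawn are set, otherwise routes to Deactivate.
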(event Custom|SpawnedActorDestroy
  (params (SpawnedActor :type Actor%20Object%20Reference))
  (if (Variables|Default|GetControlSpawned?)
    (if (Variables|Default|GetAutoRespawn?)
      (CallFunction|Activate)
      (else
        (CallFunction|Deactivate :!label _label)))
    (else
      (Utilities|IsValid SpawnedActor
        (:Is%20Valid
          (Variables|Default|SetSpawnedActor SpawnedActor)
          (goto _label))))))

(event Custom|SpawnActor
  (bind _returnvalue (Transformation|GetActorTransform))
  (bind _self self)
  (bind _size (Variables|Block|GetSize))
  (bind _form (Variables|Block|GetForm))
  (switch Utilities|FlowControl|Switch|SwitchonSpawneableActors (Variables|Default|GetActorToSpawn)
    (:NewEnumerator0
      (bind _returnvalue_2 (Game|SpawnActorfromClass "/Game/GeometricWorld/BP/Actors/BP_DestructibleBlock.BP_DestructibleBlock_C" _returnvalue "Undefined" "MultiplyWithRoot" _self _form _size 0))
      (Variables|Default|SetSpawnedActor _returnvalue_2))
    (:NewEnumerator1
      (bind _returnvalue_3 (Game|SpawnActorfromClass "/Game/GeometricWorld/BP/Actors/BP_Block.BP_Block_C" _returnvalue "Undefined" "MultiplyWithRoot" _self _form _size (Variables|Block|GetInitialLaunch) (Variables|Block|GetLight?) 0))
      (Variables|Default|SetSpawnedActor _returnvalue_3))
    (:NewEnumerator2
      (bind _returnvalue_4 (Game|SpawnActorfromClass "/Game/GeometricWorld/BP/AI/BP_DragonHead.BP_DragonHead_C" _returnvalue "Undefined" "MultiplyWithRoot" _self (Variables|Enemy|GetPatrolFromStart?) (Variables|Enemy|GetStartPatrolDelay) 0))
      (Variables|Default|SetSpawnedActor _returnvalue_4))))

(event EventActivate
  (if (Variables|Default|GetControlSpawned?)
    (Utilities|IsValid (Variables|Default|GetSpawnedActor)
      (:Is%20Valid
        (Audio|PlaySoundatLocation "/Game/GeometricWorld/SFX/Hit.Hit" (Transformation|GetWorldLocation (Actor|GetComponentbyClass (Variables|Default|GetSpawnedActor) "/Script/Engine.StaticMeshComponent")) "0, 0, 0" 0.1 0.6 0.0 "/Game/GeometricWorld/SFX/SA_Standard.SA_Standard" 0 0 0)
        (Actor|DestroyActor (Variables|Default|GetSpawnedActor))
        (Variables|Default|SetSpawnedActor 0))
      (:Is%20Not%20Valid
        _))
    (CallFunction|SpawnActor)
    (else
      (CallFunction|SpawnActor))))

(event EventDeactivate
  (Utilities|IsValid (Variables|Default|GetSpawnedActor)
    (:Is%20Valid
      (Audio|PlaySoundatLocation "/Game/GeometricWorld/SFX/Hit.Hit" (Transformation|GetWorldLocation (Actor|GetComponentbyClass (Variables|Default|GetSpawnedActor) "/Script/Engine.StaticMeshComponent")) "0, 0, 0" 0.1 0.6 0.0 "/Game/GeometricWorld/SFX/SA_Standard.SA_Standard" 0 0 0)
      (Actor|DestroyActor (Variables|Default|GetSpawnedActor))
      (Variables|Default|SetSpawnedActor 0))))

(event EventBeginPlay
  (if (Variables|Default|GetSpawnOnStart?)
    (CallFunction|Activate)))

(fn ConstructionScript)