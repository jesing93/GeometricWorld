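; BP_Block is a physics block that receives an initial launch impulse and can knock the GeometricWorld character on impact.
; Construction picks its mesh from the Form, sets a matching green material, scales it by Size, and chooses a light or heavy bounce physical material.
; Fast, strong, suitably directed hits launch the character against the block's velocity, scaled by Size.
; Fast hits also play a speed-scaled, rate-limited sound.
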(event Custom|ResetHitSound
  (Utilities|FlowControl|DoOnce false) ; enters at Reset
)

(event EventBeginPlay
  (Physics|AddImpulse (Variables|Default|GetStaticMesh) (Variables|Default|GetInitialLaunch) "None" true))

(event Collision|EventHit
  (params (MyComp :type Primitive%20Component%20Object%20Reference) (Other :type Actor%20Object%20Reference) (OtherComp :type Primitive%20Component%20Object%20Reference) (bSelfMoved :type Boolean) (HitLocation :type Vector :default "0, 0, 0") (HitNormal :type Vector :default "0, 0, 0") (NormalImpulse :type Vector :default "0, 0, 0") (Hit :type Hit%20Result%20Structure%20%28by%20ref%29))
  (bind _returnvalue (Transformation|GetVelocity))
  (if (> (Math|Vector|VectorLength _returnvalue) 5e+02)
    (if (== (Utilities|GetClass Other) "/Game/GeometricWorld/BP/Character/BP_GeometricWorldCharacter.BP_GeometricWorldCharacter_C")
      (if (and (> (Math|Vector|VectorLength NormalImpulse) 2e+04) (> (Math|Vector|VectorLength (+ (.ImpactNormal (Collision|BreakHitResult Hit)) (Math|Vector|ClampVectorSize _returnvalue -1.0 1.0))) 1.0))
        (Character|LaunchCharacter (.AsBP%20Geometric%20World%20Character (Utilities|Casting|CastToBP_GeometricWorldCharacter Other)) (* (* (* _returnvalue "-1.000000,-1.000000,-1.000000") 0.75) (Variables|Default|GetSize)) false false)))
    (Utilities|FlowControl|DoOnce false
      (:Completed
        (Audio|PlaySoundatLocation "/Game/GeometricWorld/SFX/Hit.Hit" HitLocation "0, 0, 0" (Math|Float|Clamp(Float) (/ (Math|Vector|VectorLength (Transformation|GetComponentVelocity (Variables|Default|GetStaticMesh))) 1.2e+03) 0.0 0.05) 1.0 0.0 "/Game/GeometricWorld/SFX/SA_Standard.SA_Standard" 0 0 0)
        (Utilities|FlowControl|Delay 0.32)
        (CallFunction|ResetHitSound)))))

(fn ConstructionScript
  (bind _form (Variables|Default|GetForm))
  (bind _staticmesh (Variables|Default|GetStaticMesh))
  (bind _staticmesh_2 (Variables|Default|GetStaticMesh))
  (bind _size (Variables|Default|GetSize))
  (Components|StaticMesh|SetStaticMesh (Variables|Default|GetStaticMesh) (.Value (Utilities|Map|Find (Variables|Default|GetGeometricForms) _form)))
  (if (Utilities|Enum|Equal(Enum) _form "NewEnumerator1")
    (Rendering|Material|SetMaterial _staticmesh_2 0 "/Game/GeometricWorld/Materials/MI_BasicMaterialEmmisiveGreen.MI_BasicMaterialEmmisiveGreen")
    (else
      (Rendering|Material|SetMaterial _staticmesh_2 0 "/Game/GeometricWorld/Materials/MI_BasicMaterialWEdgesGreen.MI_BasicMaterialWEdgesGreen")))
  (Transformation|SetRelativeScale3D (Variables|Default|GetStaticMesh) (Math|Vector|MakeVector _size _size _size))
  (if (Variables|Default|GetLight?)
    (Class|PrimitiveComponent|SetPhysMaterialOverride _staticmesh "/Game/GeometricWorld/Physics/PM_BouncePhysics.PM_BouncePhysics")
    (else
      (Class|PrimitiveComponent|SetPhysMaterialOverride _staticmesh "/Game/GeometricWorld/Physics/PM_HeavyBouncePhysics.PM_HeavyBouncePhysics"))))