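; BP_Spike is a hazard actor that kills the player character on contact.
; Its construction script picks the static mesh from the GeometricForms map using the Form value, then applies a red emissive material, identical in both branches of the form check.
; When the mesh begins overlapping player 0's character, it calls Death on BP_GeometricWorldCharacter.
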(event OnComponentBeginOverlap(StaticMesh)
  (params (OverlappedComponent :type Primitive%20Component%20Object%20Reference) (OtherActor :type Actor%20Object%20Reference) (OtherComp :type Primitive%20Component%20Object%20Reference) (OtherBodyIndex :type Integer) (bFromSweep :type Boolean) (SweepResult :type Hit%20Result%20Structure%20%28by%20ref%29))
  (bind _returnvalue (Game|GetPlayerCharacter 0))
  (if (== OtherActor _returnvalue)
    (Default|Death (.AsBP%20Geometric%20World%20Character (Utilities|Casting|CastToBP_GeometricWorldCharacter _returnvalue)))))

(event EventBeginPlay)

(event Collision|EventActorBeginOverlap
  (params (OtherActor :type Actor%20Object%20Reference)))

(event EventTick
  (params (DeltaSeconds :type Float%20%28single-precision%29)))

(fn ConstructionScript
  (bind _form (Variables|Default|GetForm))
  (bind _staticmesh (Variables|Default|GetStaticMesh))
  (Components|StaticMesh|SetStaticMesh (Variables|Default|GetStaticMesh) (.Value (Utilities|Map|Find (Variables|Default|GetGeometricForms) _form)))
  (if (Utilities|Enum|Equal(Enum) _form "NewEnumerator1")
    (Rendering|Material|SetMaterial _staticmesh 0 "/Game/GeometricWorld/Materials/MI_BasicMaterialEmmisiveRed.MI_BasicMaterialEmmisiveRed")
    (else
      (Rendering|Material|SetMaterial _staticmesh 0 "/Game/GeometricWorld/Materials/MI_BasicMaterialEmmisiveRed.MI_BasicMaterialEmmisiveRed"))))