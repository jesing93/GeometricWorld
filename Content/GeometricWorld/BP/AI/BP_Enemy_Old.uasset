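; BP_Enemy_Old is an AI enemy that chases a detected goal and kills the player character on contact.
; Hits on its body, eyes and yaw components, or overlaps on the body, bind an actor-hit handler at that moment, which calls Death when the other actor is the player.
; Detect starts an AI MoveTo toward the goal and sets Following, clearing the flag two seconds later without stopping the move.
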(event OnComponentHit(UpperYaw)
  (params (HitComponent :type Primitive%20Component%20Object%20Reference) (OtherActor :type Actor%20Object%20Reference) (OtherComp :type Primitive%20Component%20Object%20Reference) (NormalImpulse :type Vector :default "0, 0, 0") (Hit :type Hit%20Result%20Structure%20%28by%20ref%29))
  (Collision|AssignOnActorHit (delegate Custom|OnActorHit_Event)))

(event OnComponentHit(LowerYaw)
  (params (HitComponent :type Primitive%20Component%20Object%20Reference) (OtherActor :type Actor%20Object%20Reference) (OtherComp :type Primitive%20Component%20Object%20Reference) (NormalImpulse :type Vector :default "0, 0, 0") (Hit :type Hit%20Result%20Structure%20%28by%20ref%29))
  (Collision|AssignOnActorHit (delegate Custom|OnActorHit_Event)))

(event OnComponentBeginOverlap(Body)
  (params (OverlappedComponent :type Primitive%20Component%20Object%20Reference) (OtherActor :type Actor%20Object%20Reference) (OtherComp :type Primitive%20Component%20Object%20Reference) (OtherBodyIndex :type Integer) (bFromSweep :type Boolean) (SweepResult :type Hit%20Result%20Structure%20%28by%20ref%29))
  (Collision|AssignOnActorHit (delegate Custom|OnActorHit_Event)))

(event OnComponentHit(Body)
  (params (HitComponent :type Primitive%20Component%20Object%20Reference) (OtherActor :type Actor%20Object%20Reference) (OtherComp :type Primitive%20Component%20Object%20Reference) (NormalImpulse :type Vector :default "0, 0, 0") (Hit :type Hit%20Result%20Structure%20%28by%20ref%29))
  (Collision|AssignOnActorHit (delegate Custom|OnActorHit_Event)))

(event OnComponentHit(LeftEye)
  (params (HitComponent :type Primitive%20Component%20Object%20Reference) (OtherActor :type Actor%20Object%20Reference) (OtherComp :type Primitive%20Component%20Object%20Reference) (NormalImpulse :type Vector :default "0, 0, 0") (Hit :type Hit%20Result%20Structure%20%28by%20ref%29))
  (Collision|AssignOnActorHit (delegate Custom|OnActorHit_Event)))

(event OnComponentHit(RightEye)
  (params (HitComponent :type Primitive%20Component%20Object%20Reference) (OtherActor :type Actor%20Object%20Reference) (OtherComp :type Primitive%20Component%20Object%20Reference) (NormalImpulse :type Vector :default "0, 0, 0") (Hit :type Hit%20Result%20Structure%20%28by%20ref%29))
  (Collision|AssignOnActorHit (delegate Custom|OnActorHit_Event)))

(event Custom|OnActorHit_Event
  (params (SelfActor :type Actor%20Object%20Reference) (OtherActor :type Actor%20Object%20Reference) (NormalImpulse :type Vector) (Hit :type Hit%20Result%20Structure%20%28by%20ref%29))
  (bind _returnvalue (Game|GetPlayerCharacter 0))
  (if (== OtherActor _returnvalue)
    (Default|Death (.AsBP%20Geometric%20World%20Character (Utilities|Casting|CastToBP_GeometricWorldCharacter _returnvalue)))))

(event Custom|Detect
  (params (Goal :type Actor%20Object%20Reference))
  (Utilities|FlowControl|Sequence
    (:then_0
      (Variables|Default|SetFollowing true)
      (AI|AIMoveTo self "0, 0, 0" Goal 0.0 true))
    (:then_1
      (Utilities|FlowControl|Delay 2.0)
      (Variables|Default|SetFollowing false))))

(event EventTick
  (params (DeltaSeconds :type Float%20%28single-precision%29)))

(fn ConstructionScript)