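; BP_Pick is a collectible pickup actor for the GeometricWorld game, collected once when the player character overlaps its sphere.
; On pickup it calls PickItem on BP_GeometricWorldCharacter, spawns a spark burst at the mesh, hides the mesh and particle system, and plays a 2D sound.
; A Picked flag blocks repeat triggers, and the actor destroys itself after a short delay.
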(event OnComponentBeginOverlap(Sphere)
  (params (OverlappedComponent :type Primitive%20Component%20Object%20Reference) (OtherActor :type Actor%20Object%20Reference) (OtherComp :type Primitive%20Component%20Object%20Reference) (OtherBodyIndex :type Integer) (bFromSweep :type Boolean) (SweepResult :type Hit%20Result%20Structure%20%28by%20ref%29))
  (bind _returnvalue (Game|GetPlayerCharacter 0))
  (if (and (not (Variables|Default|GetPicked)) (== OtherActor _returnvalue))
    (Variables|Default|SetPicked true)
    (Default|PickItem (.AsBP%20Geometric%20World%20Character (Utilities|Casting|CastToBP_GeometricWorldCharacter _returnvalue)))
    (bind _returnvalue_2 (Effects|SpawnEmitteratLocation "/Game/GeometricWorld/VFX/P_SmallSparks.P_SmallSparks" (Transformation|GetWorldLocation (Variables|Default|GetStaticMesh))))
    (Variables|Default|SetPickUpParticles _returnvalue_2)
    (Rendering|SetVisibility (Variables|Default|GetStaticMesh) false false)
    (Audio|PlaySound2D "/Game/GeometricWorld/SFX/PickUp.PickUp" 1.0 1.0 0.0 0 0)
    (Utilities|FlowControl|Delay 3.0)
    (Actor|DestroyActor)))

(event EventBeginPlay)

(event Collision|EventActorBeginOverlap
  (params (OtherActor :type Actor%20Object%20Reference)))

(event EventTick
  (params (DeltaSeconds :type Float%20%28single-precision%29)))

(fn ConstructionScript)