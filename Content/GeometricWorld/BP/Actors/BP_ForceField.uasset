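; BP_ForceField is a force field barrier that opens on Activate and closes on Deactivate, guarded by an Open flag.
; Each switch toggles collision on the Movable mesh, rescales Box and swaps the NavModifier area between default and null, so navigation follows the state.
; A Timeline, played or reversed, fades Opacity on a dynamic edged orange material.
; The construction script creates that material and applies the initial state from Open.
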(event EventActivate
  (if (not (Variables|Default|GetOpen))
    (Variables|Default|SetOpen true)
    (Collision|SetCollisionEnabled (Variables|Default|GetMovable) "NoCollision")
    (Class|NavModifierComponent|SetAreaClass (Variables|Default|GetNavModifier) "/Script/NavigationSystem.NavArea_Default")
    (Transformation|SetRelativeScale3D (Variables|Default|GetBox) "0, 0, 0")
    (bind _opacitytrack (Timeline|Timeline Play)
      (:Update
        (Rendering|Material|SetScalarParameterValue (Variables|Default|GetDoorMat) "Opacity" _opacitytrack :!class /Script/Engine.MaterialInstanceDynamic)))))

(event EventDeactivate
  (if (Variables|Default|GetOpen)
    (Variables|Default|SetOpen false)
    (Collision|SetCollisionEnabled (Variables|Default|GetMovable) "QueryAndPhysics")
    (Class|NavModifierComponent|SetAreaClass (Variables|Default|GetNavModifier) "/Script/NavigationSystem.NavArea_Null")
    (Transformation|SetRelativeScale3D (Variables|Default|GetBox) "2.000000,1.000000,2.000000")
    (bind _opacitytrack (Timeline|Timeline Reverse)
      (:Update
        (Rendering|Material|SetScalarParameterValue (Variables|Default|GetDoorMat) "Opacity" _opacitytrack :!class /Script/Engine.MaterialInstanceDynamic)))))

(fn ConstructionScript
  (bind _returnvalue (Rendering|Material|CreateDynamicMaterialInstance (Variables|Default|GetMovable) 0 "/Game/GeometricWorld/Materials/MI_TransparentMaterialWEdgesOrange.MI_TransparentMaterialWEdgesOrange" "None" :!class /Script/Engine.PrimitiveComponent))
  (Variables|Default|SetDoorMat _returnvalue)
  (if (Variables|Default|GetOpen)
    (Collision|SetCollisionEnabled (Variables|Default|GetMovable) "NoCollision")
    (Transformation|SetRelativeScale3D (Variables|Default|GetBox) "0, 0, 0")
    (Rendering|Material|SetScalarParameterValue (Variables|Default|GetDoorMat) "Opacity" 0.0 :!class /Script/Engine.MaterialInstanceDynamic)
    (Class|NavModifierComponent|SetAreaClass (Variables|Default|GetNavModifier) "/Script/NavigationSystem.NavArea_Default")
    (else
      (Collision|SetCollisionEnabled (Variables|Default|GetMovable) "QueryAndPhysics")
      (Transformation|SetRelativeScale3D (Variables|Default|GetBox) "1.000000,1.000000,1.000000")
      (Rendering|Material|SetScalarParameterValue (Variables|Default|GetDoorMat) "Opacity" 1.0 :!class /Script/Engine.MaterialInstanceDynamic)
      (Class|NavModifierComponent|SetAreaClass (Variables|Default|GetNavModifier) "/Script/NavigationSystem.NavArea_Null"))))