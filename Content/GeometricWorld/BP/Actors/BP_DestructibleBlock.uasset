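; BP_DestructibleBlock is a geometric block that is removed on contact with a BP_Spike, through its owning BP_Spawner.
; The construction script picks the mesh from a form-to-mesh map, assigns a form-dependent aquamarine material and applies a uniform scale from Size.
; Other sufficiently strong impacts play a hit sound with velocity-based volume, throttled by a DoOnce that resets after a short delay.
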(event Custom|ResetHitSound
  (Utilities|FlowControl|DoOnce false) ; enters at Reset
)

(event Collision|EventHit
  (params (MyComp :type Primitive%20Component%20Object%20Reference) (Other :type Actor%20Object%20Reference) (OtherComp :type Primitive%20Component%20Object%20Reference) (bSelfMoved :type Boolean) (HitLocation :type Vector :default "0, 0, 0") (HitNormal :type Vector :default "0, 0, 0") (NormalImpulse :type Vector :default "0, 0, 0") (Hit :type Hit%20Result%20Structure%20%28by%20ref%29))
  (bind _returnvalue (Components|GetOwner))
  (if (== (Utilities|GetClass (Components|GetOwner OtherComp)) "/Game/GeometricWorld/BP/Actors/BP_Spike.BP_Spike_C")
    (Utilities|IsValid _returnvalue
      (:Is%20Valid
        (Default|SpawnedActorDestroy (.AsBP%20Spawner (Utilities|Casting|CastToBP_Spawner _returnvalue)) self)))
    (elif (> (Math|Vector|VectorLength NormalImpulse) 2e+04)
      (Utilities|FlowControl|DoOnce false
        (:Completed
          (Audio|PlaySoundatLocation "/Game/GeometricWorld/SFX/Hit.Hit" HitLocation "0, 0, 0" (Math|Float|Clamp(Float) (/ (Math|Vector|VectorLength (Transformation|GetComponentVelocity (Variables|Default|GetStaticMesh))) 1.2e+03) 0.0 0.05) 1.0 0.0 "/Game/GeometricWorld/SFX/SA_Standard.SA_Standard" 0 0 0)
          (Utilities|FlowControl|Delay 0.32)
          (CallFunction|ResetHitSound))))))

(fn ConstructionScript
  (bind _form (Variables|Default|GetForm))
  (bind _staticmesh (Variables|Default|GetStaticMesh))
  (bind _size (Variables|Default|GetSize))
  (Components|StaticMesh|SetStaticMesh (Variables|Default|GetStaticMesh) (.Value (Utilities|Map|Find (Variables|Default|GetGeometricForms) _form)))
  (if (Utilities|Enum|Equal(Enum) _form "NewEnumerator1")
    (Rendering|Material|SetMaterial _staticmesh 0 "/Game/GeometricWorld/Materials/MI_BasicMaterialEmmisiveAquamarine.MI_BasicMaterialEmmisiveAquamarine")
    (else
      (Rendering|Material|SetMaterial _staticmesh 0 "/Game/GeometricWorld/Materials/MI_BasicMaterialWEdgesAquamarine.MI_BasicMaterialWEdgesAquamarine")))
  (Transformation|SetRelativeScale3D (Variables|Default|GetStaticMesh) (Math|Vector|MakeVector _size _size _size)))